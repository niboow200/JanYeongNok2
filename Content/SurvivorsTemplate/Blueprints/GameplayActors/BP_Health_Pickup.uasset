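; Health pickup actor that restores health to the character that collects it.
; DoPickupAction sends a RestoreHealth interface message to that character with the HealthAmount value.
; MCPickupEffects spawns the health orb particle burst and plays the health sound at the pickup's location.
; The Blueprint only implements these two events and contains no overlap or trigger logic of its own.
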(event EventBeginPlay
  (|CallParentFunction) ; This node is disabled and will not be called.\nDrag off pins to build functionality.
)

(event Collision|EventActorBeginOverlap
  (params (OtherActor :type Actor%20Object%20Reference))
  (|CallParentFunction OtherActor) ; This node is disabled and will not be called.\nDrag off pins to build functionality.
)

(event EventTick
  (params (DeltaSeconds :type Float%20%28single-precision%29))
  (|CallParentFunction DeltaSeconds) ; This node is disabled and will not be called.\nDrag off pins to build functionality.
)

(event EventDoPickupAction
  (params (Character :type Actor%20Object%20Reference))
  ;[0.1094 0.1094 0.1094] Restore character Health
  (Class|ICharacterManager|RestoreHealth(Message) Character (Variables|Default|GetHealthAmount)))

(event EventMCPickupEffects
  (bind _returnvalue (Transformation|GetActorLocation))
  (Effects|SpawnEmitteratLocation "/Game/SurvivorsTemplate/Demo/Effects/FX_Archive/P_HealthOrb_Pickup.P_HealthOrb_Pickup" _returnvalue "0, 0, 0" "2.000000,2.000000,2.000000")
  (Audio|PlaySoundatLocation "/Game/SurvivorsTemplate/Demo/Sounds/Character/Cue_Health.Cue_Health" _returnvalue "0, 0, 0" 1.0 1.0 0.0 0 0 0 0))

(fn ConstructionScript
  (|CallParentFunction))